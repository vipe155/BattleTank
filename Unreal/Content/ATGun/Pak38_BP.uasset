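; Pak38_BP is an anti-tank gun actor with a tank aiming component and a floating health bar.
; On BeginPlay it initializes TankAiming with its barrel and top as turret, then passes itself to the HealthBar_BP widget as MyTank.
; Every Tick it turns the health bar widget toward the player camera so it stays readable.
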(event EventBeginPlay
  (Class|TankAimingComponent|Initialize (Variables|Default|GetTankAiming) (Variables|Default|GetBarrel) (Variables|Default|GetTop))
  (CallFunction|InitializeHealthBar))

(event EventTick
  (params (DeltaSeconds :type Float%20%28single-precision%29))
  (CallFunction|SetHealthBarRotation))

(fn ConstructionScript)

(fn InitializeHealthBar
  (bind _ashealth_bar_bp (Utilities|Casting|CastToHealthBar_BP (UserInterface|GetUserWidgetObject (Variables|Default|GetHealthBar))))
  (Variables|/Game/UI/BP/HealthBar_BP.HealthBar_BP_C|SetMyTank _ashealth_bar_bp self)
  (return))

(fn SetHealthBarRotation
  (bind _healthbar (Variables|Default|GetHealthBar))
  (Transformation|SetWorldRotation _healthbar (Math|Rotator|FindLookatRotation (Transformation|GetWorldLocation _healthbar) (Transformation|GetActorLocation (Variables|/Script/Engine.PlayerController|GetPlayerCameraManager (Game|GetPlayerController 0)))) false false))